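; Touchable storage-zone actor for the food-storing level that moves the player pawn between the overview and pantry, fridge or freezer close-ups.
; LocationNumber selects the view in ZoomLocation, which manages a height-limited BP_StoringArrow and text labels.
; Zone touches zoom only from the overview and show Portuguese hints, using flags synced across instances to shorten repeats.
; Sphere touches zoom unconditionally; unmatched numbers restore the start view.
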(event OnInputTouchBegin(ZoneMesh)
  (params (FingerIndex :type ETouchIndex%20Enum :default "Touch1") (TouchedComponent :type Primitive%20Component%20Object%20Reference))
  (CallFunction|CheckPositionandZoom (Variables|Default|GetLocationNumber)))

(event OnInputTouchBegin(Sphere)
  (params (FingerIndex :type ETouchIndex%20Enum :default "Touch1") (TouchedComponent :type Primitive%20Component%20Object%20Reference))
  (CallFunction|ZoomLocation (Variables|Default|GetLocationNumber)))

(event EventBeginPlay
  ;[1 1 1] Getting a reference to storingPawn to avoid recasts
  (Utilities|IsValid (Variables|Default|GetPawnRef)
    (:Is%20Not%20Valid
      (bind _asstoring_pawn (Utilities|Casting|CastToStoringPawn (Game|Player|GetPlayerPawn 0))
        (:then
          (Variables|Default|SetPawnRef _asstoring_pawn))
        (:CastFailed
          (Development|PrintString "you trolling you have no storing pawn"))))))

(event Collision|EventActorBeginOverlap
  (params (OtherActor :type Actor%20Object%20Reference)))

(event EventTick
  (params (DeltaSeconds :type Float%20%28single-precision%29)))

(fn ConstructionScript)

(fn ZoomLocation
  (params (LocationNumber :type Integer))
  (bind _pawnref (Variables|Default|GetPawnRef))
  (bind _defaultsceneroot (Variables|/Game/LevelsParameters/Storing/StoringPawn.StoringPawn_C|GetDefaultSceneRoot _pawnref))
  (switch int LocationNumber
    (:Default
      ;[1 1 1] Start position
      (CallFunction|StartPositiioin _defaultsceneroot))
    (:1
      ;[1 1 1] Pantry
      (Transformation|SetRelativeLocation _defaultsceneroot "588.713169,-550.673519,200.000000" false false)
      (bind _outactors (Actor|GetAllActorsOfClass "/Game/LevelsParameters/Storing/BP_StoringArrow.BP_StoringArrow_C"))
      (if (Utilities|Array|IsEmpty _outactors)
        ;[1 1 1] Rever valores StoringLocations
        (Game|SpawnActorfromClass "/Game/LevelsParameters/Storing/BP_StoringArrow.BP_StoringArrow_C" (Math|Transform|MakeTransform "972.506804,-320.589387,20.720000") "Undefined" 0 (Variables|Default|GetLocationNumber) 2.8e+02 2e+01 1.0 0)
        (bind _outactors_2 (Actor|GetAllActorsOfClass "/Script/Engine.TextRenderActor" :!label _label))
        (for _array_element _outactors_2
          (Rendering|SetVisibility (Variables|/Script/Engine.TextRenderActor|GetTextRender _array_element) true true))))
    (:2
      ;[1 1 1] Fridge
      (Transformation|SetRelativeLocation _defaultsceneroot "588.713169,-4.613227,440.000000" false false)
      (bind _outactors_3 (Actor|GetAllActorsOfClass "/Game/LevelsParameters/Storing/BP_StoringArrow.BP_StoringArrow_C"))
      (if (Utilities|Array|IsEmpty _outactors_3)
        _
        (else
          (Actor|DestroyActor _outactors_3)))
      (Game|SpawnActorfromClass "/Game/LevelsParameters/Storing/BP_StoringArrow.BP_StoringArrow_C" (Math|Transform|MakeTransform "972.506804,203.000000,230.720000") "Undefined" 0 (Variables|Default|GetLocationNumber) 524.0 2.3e+02 1.0 0)
      (goto _label))
    (:3
      ;[1 1 1] Freezer
      (Transformation|SetRelativeLocation _defaultsceneroot "588.713169,-4.613227,200.000000" false false)
      (bind _outactors_4 (Actor|GetAllActorsOfClass "/Game/LevelsParameters/Storing/BP_StoringArrow.BP_StoringArrow_C"))
      (if (Utilities|Array|IsEmpty _outactors_4)
        _
        (else
          (Actor|DestroyActor _outactors_4)))
      (Game|SpawnActorfromClass "/Game/LevelsParameters/Storing/BP_StoringArrow.BP_StoringArrow_C" (Math|Transform|MakeTransform "972.506804,203.000000,20.720000") "Undefined" 0 (Variables|Default|GetLocationNumber) 203.0 2e+01 1.0 0)
      (goto _label))))

(fn CheckPositionandZoom
  (params (LocationNumber :type Integer))
  (if (< (.x (Transformation|GetActorLocation (Game|Player|GetPlayerPawn 0))) 124.0)
    (CallFunction|ZoomLocation LocationNumber)
    (if (== (Variables|/Game/LevelsParameters/Storing/StoringPawn.StoringPawn_C|GetFoodRef (Variables|Default|GetPawnRef)) 0)
      (Utilities|FlowControl|Sequence
        (:then_0
          (bind _foundwidgets (Widget|GetAllWidgetsOfClass "/Game/UIElements/WBP_CommonUI.WBP_CommonUI_C" true))
          (Variables|/Game/UIElements/WBP_CommonUI.WBP_CommonUI_C|SetDialogueString (Utilities|Array|Get(acopy) _foundwidgets) "Antes de entrares na zona de arrumação seleciona a comida do cesto, para voltares atrás tens o círculo à esquerda.")
          (Widget|SetVisibility (Variables|/Game/UIElements/WBP_CommonUI.WBP_CommonUI_C|GetDialogueContainer (Utilities|Array|Get(acopy) _foundwidgets)) "Visible")
          (Default|SetImage (Utilities|Array|Get(acopy) _foundwidgets) "Back")
          (Widget|SetVisibility (Variables|/Game/UIElements/WBP_CommonUI.WBP_CommonUI_C|GetChefimgButton (Utilities|Array|Get(acopy) _foundwidgets)) "Hidden")))
      (else
        (Utilities|FlowControl|Sequence
          (:then_1
            (if (Variables|Default|GetC1)
              (bind _foundwidgets_2 (Widget|GetAllWidgetsOfClass "/Game/UIElements/WBP_CommonUI.WBP_CommonUI_C" true))
              (Variables|/Game/UIElements/WBP_CommonUI.WBP_CommonUI_C|SetDialogueString (Utilities|Array|Get(acopy) _foundwidgets_2) "Tem atenção à comida e às prateleiras clica na comida quando quiseres arrumá-la, para voltar atrás tens o círculo à esquerda.")
              (CallFunction|ShowBackButton :!label _label)
              (Default|StartBlinking (Utilities|Array|Get(acopy) (stale _foundwidgets_4)))
              (else
                (bind _foundwidgets_3 (Widget|GetAllWidgetsOfClass "/Game/UIElements/WBP_CommonUI.WBP_CommonUI_C" true))
                (Variables|/Game/UIElements/WBP_CommonUI.WBP_CommonUI_C|SetDialogueString (Utilities|Array|Get(acopy) _foundwidgets_3) "Tem atenção à comida e às prateleiras clica na comida quando quiseres arrumá-la, para voltar atrás tens o círculo à esquerda.")
                (Widget|SetVisibility (Variables|/Game/UIElements/WBP_CommonUI.WBP_CommonUI_C|GetDialogueContainer (Utilities|Array|Get(acopy) _foundwidgets_3)) "Visible")
                (Default|SetImage (Utilities|Array|Get(acopy) _foundwidgets_3) "Back")
                (Widget|SetVisibility (Variables|/Game/UIElements/WBP_CommonUI.WBP_CommonUI_C|GetChefimgButton (Utilities|Array|Get(acopy) _foundwidgets_3)) "Hidden")
                (Variables|Default|SetC1 true)
                (bind _outactors (Actor|GetAllActorsOfClass "BP_SelectArea_C"))
                (for _array_element _outactors
                  (Variables|BP_SelectArea_C|SetC1 _array_element true))))))))
    (else
      (Utilities|FlowControl|Sequence
        (:then_1
          (if (Variables|Default|GetC2)
            (bind _foundwidgets_4 (Widget|GetAllWidgetsOfClass "/Game/UIElements/WBP_CommonUI.WBP_CommonUI_C" true))
            (Variables|/Game/UIElements/WBP_CommonUI.WBP_CommonUI_C|SetDialogueString (Utilities|Array|Get(acopy) _foundwidgets_4) "Volta atrás clicando no círculo à esquerda com a seta, para arrumares a comida clica na comida, tem atenção à posição da seta.")
            (goto _label)
            (else
              (bind _foundwidgets_5 (Widget|GetAllWidgetsOfClass "/Game/UIElements/WBP_CommonUI.WBP_CommonUI_C" true))
              (Variables|/Game/UIElements/WBP_CommonUI.WBP_CommonUI_C|SetDialogueString (Utilities|Array|Get(acopy) _foundwidgets_5) "Volta atrás clicando no círculo à esquerda com a seta, para arrumares a comida clica na comida, tem atenção à posição da seta.")
              (Widget|SetVisibility (Variables|/Game/UIElements/WBP_CommonUI.WBP_CommonUI_C|GetDialogueContainer (Utilities|Array|Get(acopy) _foundwidgets_5)) "Visible")
              (Default|SetImage (Utilities|Array|Get(acopy) _foundwidgets_5) "Back")
              (Widget|SetVisibility (Variables|/Game/UIElements/WBP_CommonUI.WBP_CommonUI_C|GetChefimgButton (Utilities|Array|Get(acopy) _foundwidgets_5)) "Hidden")
              (Variables|Default|SetC2 true)
              (bind _outactors_2 (Actor|GetAllActorsOfClass "BP_SelectArea_C"))
              (for _array_element_2 _outactors_2
                (Variables|BP_SelectArea_C|SetC2 _array_element_2 true)))))))))

(fn StartPositiioin
  (params (SelfComponent :type Scene%20Component%20Object%20Reference))
  (Transformation|SetRelativeLocation SelfComponent "123.508975,-13.768993,200.000000" false false)
  (bind _outactors (Actor|GetAllActorsOfClass "/Game/LevelsParameters/Storing/BP_StoringArrow.BP_StoringArrow_C"))
  (Actor|DestroyActor _outactors)
  (bind _outactors_2 (Actor|GetAllActorsOfClass "/Script/Engine.TextRenderActor"))
  (for _array_element _outactors_2
    (Rendering|SetVisibility (Variables|/Script/Engine.TextRenderActor|GetTextRender _array_element) false true)
    (bind _foundwidgets (Widget|GetAllWidgetsOfClass "/Game/UIElements/WBP_CommonUI.WBP_CommonUI_C" true))
    (Widget|SetVisibility (Variables|/Game/UIElements/WBP_CommonUI.WBP_CommonUI_C|GetBackOrConfirmButton (Utilities|Array|Get(acopy) _foundwidgets)) "Hidden")
    (bind _outactors_3 (Actor|GetAllActorsOfClass "BP_SelectArea_C"))
    (for _array_element_2 _outactors_3
      (if (== (Variables|BP_SelectArea_C|GetLocationNumber _array_element_2) 546)
        (Rendering|SetVisibility (Variables|BP_SelectArea_C|GetZoneMesh _array_element_2) false true)
        (CallFunction|DecreaseExpiryWidgetSize)))))

(fn DecreaseExpiryWidgetSize
  (bind _foundwidgets (Widget|GetAllWidgetsOfClass "/Game/UIElements/WBP_Expiry.WBP_Expiry_C" true))
  (for _array_element _foundwidgets
    (Class|UserWidget|SetDesiredSizeinViewport _array_element "(X=50.000000,Y=50.000000)")))

(fn IncreaseExpiryWidgetSize
  (bind _outactors (Actor|GetAllActorsOfClass "/Game/LevelsParameters/Storing/BP_StoredFood.BP_StoredFood_C"))
  (for _array_element _outactors
    (Development|PrintString (Utilities|GetDisplayName (UserInterface|GetWidget (Variables|/Game/LevelsParameters/Storing/BP_StoredFood.BP_StoredFood_C|GetExpiryProgressBar _array_element))))
    (Class|CanvasPanelSlot|SetSize (Class|WidgetLayoutLibrary|SlotasCanvasSlot (UserInterface|GetWidget (Variables|/Game/LevelsParameters/Storing/BP_StoredFood.BP_StoredFood_C|GetExpiryProgressBar _array_element))) "(X=500.000000,Y=500.000000)")))

(fn ShowBackButton
  (bind _foundwidgets (Widget|GetAllWidgetsOfClass "/Game/UIElements/WBP_CommonUI.WBP_CommonUI_C" true))
  (Widget|SetVisibility (Variables|/Game/UIElements/WBP_CommonUI.WBP_CommonUI_C|GetBackOrConfirmButton (Utilities|Array|Get(acopy) _foundwidgets)) "Visible")
  (Default|BlinkIcon (Utilities|Array|Get(acopy) _foundwidgets)))