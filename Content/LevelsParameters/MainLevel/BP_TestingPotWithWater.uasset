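; Selectable pot-with-water cooking tool, apparently a test variant, for a cooking game about food waste.
; On BeginPlay it derives its tool type from the mesh name and gets the slicing pawn; Tick scales the water's height from WaterHeight.
; Touching it moves it to the cooking position, destroys other selectable cook tools and advances the pawn's step.
; If no food choices exist, it spawns them through SlicingManager and shows a Portuguese food-waste prompt.
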(event OnInputTouchBegin(Pot)
  (params (FingerIndex :type ETouchIndex%20Enum :default "Touch1") (TouchedComponent :type Primitive%20Component%20Object%20Reference))
  (bind _pawnref (Variables|Default|GetPawnRef))
  (bind _slicingmanager (Variables|/Game/LevelsParameters/SlicingTesting/UnrealExample/SliceGamePawn.SliceGamePawn_C|GetSlicingManager _pawnref))
  (bind _slicingfoodcount (Variables|/Game/LevelsParameters/SlicingTesting/Structures/Slicing_Manager.Slicing_Manager_C|GetSlicingFoodCount _slicingmanager))
  (CallFunction|MovetoCookPosition&ClearOthers)
  (Variables|/Game/LevelsParameters/Cooking/Structures/Cooking_Manager.Cooking_Manager_C|SetActiveCookingFood (Variables|/Game/LevelsParameters/SlicingTesting/UnrealExample/SliceGamePawn.SliceGamePawn_C|GetCookingManager _pawnref) (Variables|Default|GetCookingFoodNoNeed))
  (Math|Integer|IncrementInt (Variables|/Game/LevelsParameters/SlicingTesting/UnrealExample/SliceGamePawn.SliceGamePawn_C|GetCurrentStep _pawnref)
    (:%20%20
      (bind _outactors (Actor|GetAllActorsOfClass "/Game/LevelsParameters/SlicingTesting/BP_SelectSliceFood.BP_SelectSliceFood_C"))
      (if (Utilities|Array|IsEmpty _outactors)
        (Default|SpawnLevelFood _slicingmanager (- _slicingfoodcount 1))
        (Default|DecreaseFoodSpawn _slicingmanager _slicingfoodcount)
        (bind _foundwidgets (Widget|GetAllWidgetsOfClass "/Game/UIElements/WBP_CommonUI.WBP_CommonUI_C" true))
        (Variables|/Game/UIElements/WBP_CommonUI.WBP_CommonUI_C|SetDialogueString (Utilities|Array|Get(acopy) _foundwidgets) "Escolhe a comida que vai trazer mais benefícios para combater o desperdício alimentar")
        (Widget|SetVisibility (Variables|/Game/UIElements/WBP_CommonUI.WBP_CommonUI_C|GetDialogueContainer (Utilities|Array|Get(acopy) _foundwidgets)) "Visible")))))

(event EventBeginPlay
  (CallFunction|SetToolType)
  (Utilities|IsValid (Variables|Default|GetPawnRef)
    (:Is%20Not%20Valid
      (bind _asslice_game_pawn (CallFunction|GetSlicingPawn))
      (Variables|Default|SetPawnRef _asslice_game_pawn))))

(event Collision|EventActorBeginOverlap
  (params (OtherActor :type Actor%20Object%20Reference)))

(event EventTick
  (params (DeltaSeconds :type Float%20%28single-precision%29))
  (bind _water (Variables|Default|GetWater))
  (bind _returnvalue (Transformation|GetWorldScale _water))
  (Transformation|SetWorldScale3D _water (Math|Vector|MakeVector (.x _returnvalue) (.y _returnvalue) (Variables|Default|GetWaterHeight))))

(fn ConstructionScript)

(fn MovetoCookPosition&ClearOthers
  (CallFunction|SetPositionCookTool "NewEnumerator0")
  (bind _outactors (Actor|GetAllActorsOfClass "/Game/LevelsParameters/Cooking/BP_SelectCookTool.BP_SelectCookTool_C"))
  (for _array_element _outactors
    (if (not (== _array_element self))
      (Actor|DestroyActor _array_element))))

(fn SpawnProcFood
  (Game|SpawnActorfromClass "/Game/LevelsParameters/SlicingTesting/BP_NewProcComp.BP_NewProcComp_C" (Math|Transform|MakeTransform "929.884911,-15.831220,114.126350" "0, 0, 0" (Math|Vector|MakeVector 0.0 0.0 0.0)) "Undefined" 0 0 false 0))

(fn SetPositionCookTool
  (params (Selection :type ECookToolType%20Enum :default "NewEnumerator0"))
  (bind _rootcomponent (Variables|Transformation|GetRootComponent))
  (switch Utilities|FlowControl|Switch|SwitchonECookToolType Selection
    (:NewEnumerator0
      ;[1 1 1] Pot With water and without water have different offsets
      (if (Utilities|Enum|Equal(Enum) (Utilities|GetDisplayName (Variables|/Script/Engine.StaticMeshComponent|GetStaticMesh (Variables|Default|GetPot))) "PotWater")
        (Transformation|SetRelativeLocation _rootcomponent "986.226500,212.681345,103.000000" false false)
        (else
          (Transformation|SetRelativeLocation _rootcomponent "986.226500,212.681345,103.000000" false false))))
    (:NewEnumerator1
      (Transformation|SetRelativeLocation _rootcomponent "986.226500,212.681345,92.000000" false false))
    (:NewEnumerator2
      (Transformation|SetRelativeLocation _rootcomponent "986.226500,212.681345,92.000000" false false))))

(fn SetToolType
  (switch string (Utilities|GetDisplayName (Variables|/Script/Engine.StaticMeshComponent|GetStaticMesh (Variables|Default|GetPot)))
    (:Pan
      (Variables|Default|SetToolType "NewEnumerator2" :!label _label))
    (:PanWater
      (goto _label))
    (:Pot
      (Variables|Default|SetToolType "NewEnumerator0" :!label _label_2))
    (:PotWater
      (goto _label_2))
    (:Plate
      (Variables|Default|SetToolType "NewEnumerator1"))))