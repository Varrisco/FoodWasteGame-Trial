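; Compost bin for the main level that collects bad food and rewards XP when the player taps the bucket to empty it.
; AddComposting drops a short-lived physics food prop and starts a timer syncing fill height to the GameInstance composting count.
; A fast looping timer applies that height as the filling mesh's Z scale.
; Tapping clears the count and shows a result widget with sound; a box overlap toggles the text label.
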(event OnComponentBeginOverlap(Box)
  (params (OverlappedComponent :type Primitive%20Component%20Object%20Reference) (OtherActor :type Actor%20Object%20Reference) (OtherComp :type Primitive%20Component%20Object%20Reference) (OtherBodyIndex :type Integer) (bFromSweep :type Boolean) (SweepResult :type Hit%20Result%20Structure%20%28by%20ref%29))
  (Rendering|SetVisibility (Variables|Default|GetTextRender) true true))

(event OnComponentEndOverlap(Box)
  (params (OverlappedComponent :type Primitive%20Component%20Object%20Reference) (OtherActor :type Actor%20Object%20Reference) (OtherComp :type Primitive%20Component%20Object%20Reference) (OtherBodyIndex :type Integer))
  (Rendering|SetVisibility (Variables|Default|GetTextRender) false true))

(event OnInputTouchBegin(Bucket)
  (params (FingerIndex :type ETouchIndex%20Enum :default "Touch1") (TouchedComponent :type Primitive%20Component%20Object%20Reference))
  ;[1 1 1] Add SFX
  (if (> (Variables|Default|GetCompAdded) 0)
    (Variables|Default|SetZHeight 1.0)
    (bind _asbp_main_game_instance (CallFunction|GetGameInstance))
    (CallFunction|AddXP (Variables|Default|GetCompAdded))
    (Default|ClearComposting _asbp_main_game_instance)
    (Variables|Default|SetCompAdded 0)
    (bind _returnvalue (UserInterface|CreateWidget "/Game/UIElements/WBP_CleanedComposting.WBP_CleanedComposting_C"))
    (UserInterface|Viewport|AddtoViewport _returnvalue 0)
    (Audio|PlaySoundatLocation "/Game/LevelsParameters/MainLevel/SFX/TrashSound.TrashSound" "1097.517689,3014.547870,51.053898" "0, 0, 0" 1.0 1.0 0.0 0 0 0 0)
    (else
      (bind _foundwidgets (Widget|GetAllWidgetsOfClass "/Game/UIElements/WBP_CleanedComposting.WBP_CleanedComposting_C" true))
      (if (<= (Utilities|Array|Length _foundwidgets) 0)
        (bind _returnvalue_2 (UserInterface|CreateWidget "/Game/UIElements/WBP_CleanedComposting.WBP_CleanedComposting_C" 0 true))
        (UserInterface|Viewport|AddtoViewport _returnvalue_2 0)
        (Audio|PlaySoundatLocation "/Game/LevelsParameters/MainLevel/Fail.Fail" "1097.517689,3014.547870,51.053898" "0, 0, 0" 1.0 1.0 0.0 0 0 0 0)))))

(event Custom|StartChecking
  (Utilities|Time|SetTimerbyEvent (delegate Custom|CheckZHeight) 0.01 true))

(event Custom|CheckZHeight
  (CallFunction|UpdateZHeightMesh))

(event Custom|IncreaseHeight
  (CallFunction|DoubleCheckZHeight)
  (Utilities|FlowControl|Delay 2.0)
  (Math|Integer|IncrementInt (Variables|Default|GetCompAdded)))

(event Custom|DoubleCheckZHeight
  (Utilities|Time|SetTimerbyEvent (delegate Custom|Update) 1.0 true))

(event Custom|Update
  (bind _asbp_main_game_instance (CallFunction|GetGameInstance))
  (if (not (== (Variables|Default|GetCompAdded) (Variables|/Game/TopDown/Blueprints/BP_MainGameInstance.BP_MainGameInstance_C|GetComposting _asbp_main_game_instance)))
    (Variables|Default|SetZHeight (+ (* (Math|Conversions|ToFloat(Integer) (Variables|/Game/TopDown/Blueprints/BP_MainGameInstance.BP_MainGameInstance_C|GetComposting _asbp_main_game_instance)) 0.15) 1.0))
    (Variables|Default|SetCompAdded (Variables|/Game/TopDown/Blueprints/BP_MainGameInstance.BP_MainGameInstance_C|GetComposting _asbp_main_game_instance))))

(event EventBeginPlay
  (CallFunction|CheckPreviousCompostingLevel)
  (CallFunction|StartChecking))

(event Collision|EventActorBeginOverlap
  (params (OtherActor :type Actor%20Object%20Reference)))

(event EventTick
  (params (DeltaSeconds :type Float%20%28single-precision%29)))

(fn ConstructionScript)

(fn UpdateZHeightMesh
  (Transformation|SetWorldScale3D (Variables|Default|GetCompostingFilling) (Math|Vector|MakeVector 1.0 1.0 (Variables|Default|GetZHeight))))

(fn AddComposting
  (params (Mesh :type Static%20Mesh%20Object%20Reference))
  (bind _self self)
  (bind _returnvalue (Transformation|GetActorTransform _self))
  (bind _returnvalue_2 (Game|SpawnActorfromClass "/Game/LevelsParameters/MainLevel/BP_BadFood.BP_BadFood_C" (Math|Transform|MakeTransform (Math|Vector|MakeVector (.x (.location _returnvalue)) (.y (.location _returnvalue)) (+ (.z (.location _returnvalue)) 1e+01)) (.rotation _returnvalue) "0.500000,0.500000,0.500000") "Undefined" 0 Mesh 0))
  (Physics|SetSimulatePhysics (Variables|/Game/LevelsParameters/MainLevel/BP_BadFood.BP_BadFood_C|GetCube _returnvalue_2) true)
  (Rendering|Material|SetMaterial (Variables|/Game/LevelsParameters/MainLevel/BP_BadFood.BP_BadFood_C|GetCube _returnvalue_2) 0 "/Game/LevelsParameters/SlicingTesting/UnrealExample/M_BadFood.M_BadFood")
  (Actor|SetLifeSpan _returnvalue_2 2.0)
  (CallFunction|IncreaseHeight))

(fn CheckPreviousCompostingLevel
  (bind _asbp_main_game_instance (CallFunction|GetGameInstance))
  (Variables|Default|SetCompAdded (Variables|/Game/TopDown/Blueprints/BP_MainGameInstance.BP_MainGameInstance_C|GetComposting _asbp_main_game_instance))
  (Variables|Default|SetZHeight (+ (* (Math|Conversions|ToFloat(Integer) (Variables|/Game/TopDown/Blueprints/BP_MainGameInstance.BP_MainGameInstance_C|GetComposting _asbp_main_game_instance)) 0.15) (Variables|Default|GetZHeight))))

(fn IncreaseZHeight
  (Variables|Default|SetZHeight (+ (Variables|Default|GetZHeight) 0.15)))

(fn AddXP
  (params (Pieces :type Integer))
  (bind _asbp_top_down_character (CallFunction|GetBPTopDownCharacter))
  (Default|GetBonusXp (Variables|/Game/TopDown/Blueprints/BP_TopDownCharacter.BP_TopDownCharacter_C|GetLevelingComponent _asbp_top_down_character) (/ (Math|Conversions|ToFloat(Integer) Pieces) 2.0))
  (return))