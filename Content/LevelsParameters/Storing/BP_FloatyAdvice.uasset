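; Floating food-storage tip actor that shows a piece of advice in the common UI dialogue when touched.
; On BeginPlay it loads a random mesh and tip from TipsDataTable, then starts a fast looping timer.
; The timer slides the mesh back and forth along relative Y, picking a new random row at each end.
; Touching the mesh plays a sound and writes the current tip into WBP_CommonUI.
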(event OnInputTouchBegin(StaticMesh)
  (params (FingerIndex :type ETouchIndex%20Enum :default "Touch1") (TouchedComponent :type Primitive%20Component%20Object%20Reference))
  (Audio|PlaySound2D "/Game/LevelsParameters/InteractFood.InteractFood" 1.0 1.0 0.0 0 0)
  (bind _foundwidgets (Widget|GetAllWidgetsOfClass "/Game/UIElements/WBP_CommonUI.WBP_CommonUI_C" true))
  (Variables|/Game/UIElements/WBP_CommonUI.WBP_CommonUI_C|SetDialogueString (Utilities|Array|Get(acopy) _foundwidgets) (Variables|Default|GetTip))
  (Widget|SetVisibility (Variables|/Game/UIElements/WBP_CommonUI.WBP_CommonUI_C|GetDialogueContainer (Utilities|Array|Get(acopy) _foundwidgets)) "Visible"))

(event Custom|MoveObject
  (CallFunction|MovementFunction))

(event Custom|StartObjectMov
  (Utilities|Time|SetTimerbyEvent (delegate Custom|MoveObject) 0.0018 true) ; First time
)

(event EventBeginPlay
  (bind _outrownames (DataTable|GetDataTableRowNames "/Game/LevelsParameters/Storing/Structures/TipsDataTable.TipsDataTable"))
  (bind _returnvalue (Utilities|GetDataTableRow "/Game/LevelsParameters/Storing/Structures/TipsDataTable.TipsDataTable" (.OutItem (Utilities|Array|Random _outrownames)))
    (:then
      (Components|StaticMesh|SetStaticMesh (Variables|Default|GetStaticMesh) (.Mesh (Utilities|Struct|BreakTipsStruct _returnvalue)))
      (Variables|Default|SetTip (Utilities|String|ToString(Text) (.Tip (Utilities|Struct|BreakTipsStruct _returnvalue))))
      (CallFunction|StartObjectMov))))

(event Collision|EventActorBeginOverlap
  (params (OtherActor :type Actor%20Object%20Reference)))

(event EventTick
  (params (DeltaSeconds :type Float%20%28single-precision%29)))

(fn ConstructionScript)

(fn MovementFunction
  (bind _staticmesh (Variables|Default|GetStaticMesh))
  (bind _returnvalue (Transformation|GetRelativeTransform _staticmesh))
  (if (Variables|Default|GetisMovUp)
    (if (== (Variables|Default|GetEndPosition) (Variables|Default|GetCurrentYPosition))
      (Variables|Default|SetisMovUp false)
      (CallFunction|SetMeshandTip)
      (else
        (Variables|Default|SetCurrentYPosition (+ (Variables|Default|GetCurrentYPosition) 0.25))
        (Transformation|SetRelativeLocation _staticmesh (Math|Vector|MakeVector (.x (.location _returnvalue)) (Variables|Default|GetCurrentYPosition) (.z (.location _returnvalue))) false false :!label _label)))
    (elif (== (Variables|Default|GetStartPosition) (Variables|Default|GetCurrentYPosition))
      (Variables|Default|SetisMovUp true)
      (CallFunction|SetMeshandTip)
      (else
        (Variables|Default|SetCurrentYPosition (- (Variables|Default|GetCurrentYPosition) 0.25))
        (goto _label)))))

(fn SetMeshandTip
  (bind _outrownames (DataTable|GetDataTableRowNames "/Game/LevelsParameters/Storing/Structures/TipsDataTable.TipsDataTable"))
  (bind _returnvalue (Utilities|GetDataTableRow "/Game/LevelsParameters/Storing/Structures/TipsDataTable.TipsDataTable" (.OutItem (Utilities|Array|Random _outrownames)))
    (:then
      (Variables|Default|SetCurrentIndex (.OutIndex (Utilities|Array|Random _outrownames)))
      (Components|StaticMesh|SetStaticMesh (Variables|Default|GetStaticMesh) (.Mesh (Utilities|Struct|BreakTipsStruct _returnvalue)))
      (Variables|Default|SetTip (Utilities|String|ToString(Text) (.Tip (Utilities|Struct|BreakTipsStruct _returnvalue)))))))