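; Evaluation plate actor that lets the player receive their final evaluation in the main level.
; Entering its box shows Chef Olivia's dialogue in WBP_CommonUI with a Portuguese prompt to click the plate, gated by a DoOnce that resets on exit.
; Touching the plate plays a sound, calls the final score and highlight function on the MainHUB_Manager found at BeginPlay, then removes the actor through a very short lifespan.
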(event OnComponentBeginOverlap(Box)
  (params (OverlappedComponent :type Primitive%20Component%20Object%20Reference) (OtherActor :type Actor%20Object%20Reference) (OtherComp :type Primitive%20Component%20Object%20Reference) (OtherBodyIndex :type Integer) (bFromSweep :type Boolean) (SweepResult :type Hit%20Result%20Structure%20%28by%20ref%29))
  (Utilities|FlowControl|DoOnce false
    (:Completed
      (bind _foundwidgets (Widget|GetAllWidgetsOfClass "/Game/UIElements/WBP_CommonUI.WBP_CommonUI_C" true))
      (Widget|SetVisibility (Variables|/Game/UIElements/WBP_CommonUI.WBP_CommonUI_C|GetDialogueContainer (Utilities|Array|Get(acopy) _foundwidgets)) "Visible")
      ;[1 1 1] Make recipe data table
      (Variables|/Game/UIElements/WBP_CommonUI.WBP_CommonUI_C|SetDialogueString (Utilities|Array|Get(acopy) _foundwidgets) "Clica no prato que está na mesa para receberes a avaliação final."))))

(event OnComponentEndOverlap(Box)
  (params (OverlappedComponent :type Primitive%20Component%20Object%20Reference) (OtherActor :type Actor%20Object%20Reference) (OtherComp :type Primitive%20Component%20Object%20Reference) (OtherBodyIndex :type Integer))
  (Utilities|FlowControl|DoOnce false) ; enters at Reset
)

(event OnInputTouchBegin(Plate)
  (params (FingerIndex :type ETouchIndex%20Enum :default "Touch1") (TouchedComponent :type Primitive%20Component%20Object%20Reference))
  (Audio|PlaySound2D "/Game/LevelsParameters/InteractFood2.InteractFood2" 1.0 1.0 0.0 0 0)
  (Default|GetFinalEvaluationScoreandHighlight (Variables|Default|GetMainHUBManagerRef))
  (Actor|SetLifeSpan 0.01))

(event EventBeginPlay
  (bind _outactors (Actor|GetAllActorsOfClass "/Game/LevelsParameters/MainLevel/MainHUB_Manager.MainHUB_Manager_C"))
  (Variables|Default|SetMainHUBManagerRef (Utilities|Array|Get(acopy) _outactors)))

(event Collision|EventActorBeginOverlap
  (params (OtherActor :type Actor%20Object%20Reference)))

(event EventTick
  (params (DeltaSeconds :type Float%20%28single-precision%29)))

(fn ConstructionScript)