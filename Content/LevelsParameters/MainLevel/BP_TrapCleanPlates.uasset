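; BP_TrapCleanPlates is a trigger actor that shows the WBP_CleaningPlates widget while its Box is overlapped, removing it when the overlap ends.
; RemoveFoodGameInstance drops the first entry from the food data, expiry and stored-zone arrays in BP_MainGameInstance.
; EnableSlicingLevel finds the slicing level-change zone by display name, unhides and repositions it, then clears WBP_ChangeLevel widgets as a display workaround.
; Neither function is called within this Blueprint.
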(event OnComponentBeginOverlap(Box)
  (params (OverlappedComponent :type Primitive%20Component%20Object%20Reference) (OtherActor :type Actor%20Object%20Reference) (OtherComp :type Primitive%20Component%20Object%20Reference) (OtherBodyIndex :type Integer) (bFromSweep :type Boolean) (SweepResult :type Hit%20Result%20Structure%20%28by%20ref%29))
  (bind _returnvalue (UserInterface|CreateWidget "/Game/UIElements/WBP_CleaningPlates.WBP_CleaningPlates_C"))
  (UserInterface|Viewport|AddtoViewport _returnvalue 0))

(event OnComponentEndOverlap(Box)
  (params (OverlappedComponent :type Primitive%20Component%20Object%20Reference) (OtherActor :type Actor%20Object%20Reference) (OtherComp :type Primitive%20Component%20Object%20Reference) (OtherBodyIndex :type Integer))
  (Widget|RemovefromParent (stale OnComponentBeginOverlap(Box) _returnvalue)))

(event EventBeginPlay)

(event Collision|EventActorBeginOverlap
  (params (OtherActor :type Actor%20Object%20Reference)))

(event EventTick
  (params (DeltaSeconds :type Float%20%28single-precision%29)))

(fn ConstructionScript)

(fn RemoveFoodGameInstance
  (bind _asbp_main_game_instance (Utilities|Casting|CastToBP_MainGameInstance (Game|GetGameInstance)))
  (Utilities|Array|RemoveIndex (Variables|/Game/TopDown/Blueprints/BP_MainGameInstance.BP_MainGameInstance_C|GetFoodDataElement _asbp_main_game_instance))
  (Utilities|Array|RemoveIndex (Variables|/Game/TopDown/Blueprints/BP_MainGameInstance.BP_MainGameInstance_C|GetFoodExpiryElement _asbp_main_game_instance))
  (Utilities|Array|RemoveIndex (Variables|/Game/TopDown/Blueprints/BP_MainGameInstance.BP_MainGameInstance_C|GetStoredZoneString _asbp_main_game_instance))
  (return _asbp_main_game_instance))

(fn EnableSlicingLevel
  (bind _outactors (Actor|GetAllActorsOfClass "/Game/TopDown/Blueprints/BP_ChangeLevelZone.BP_ChangeLevelZone_C"))
  (for _array_element _outactors
    (if (Utilities|Enum|Equal(Enum) (Utilities|GetDisplayName _array_element) "BP_ChangeLevelSlicing")
      (Rendering|SetActorHiddenInGame _array_element false)
      (Transformation|SetWorldLocation (Variables|/Game/TopDown/Blueprints/BP_ChangeLevelZone.BP_ChangeLevelZone_C|GetDefaultSceneRoot _array_element) "587.667041,3200.000073,53.823700" false false)
      ;[1 1 1] Little fix to not show up on screen o.O
      (bind _foundwidgets (Widget|GetAllWidgetsOfClass "/Game/UIElements/WBP_ChangeLevel.WBP_ChangeLevel_C" true))
      (for _array_element_2 _foundwidgets
        (Widget|RemovefromParent _array_element_2))))
  (return))