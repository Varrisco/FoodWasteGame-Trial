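; BP_StoredFood is the food item actor shown on a shelf in the storing level.
; On BeginPlay it caches the player's StoringPawn and copies the static mesh and first material from that pawn's FoodRef.
; SpawnOnShelf places it at a fixed X with the given Y and lowered Z, at double scale.
; ZAxisAdjustment selects a height offset for pantry, fridge or freezer, currently identical for all and unused by SpawnOnShelf.
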(event EventBeginPlay
  (bind _staticmesh (Variables|Default|GetStaticMesh))
  ;[1 1 1] Getting a reference to storingPawn to avoid recasts
  (Utilities|IsValid (Variables|Default|GetPawnRef)
    (:Is%20Not%20Valid
      (bind _asstoring_pawn (Utilities|Casting|CastToStoringPawn (Game|Player|GetPlayerPawn 0))
        (:then
          (Variables|Default|SetPawnRef _asstoring_pawn)
          (Components|StaticMesh|SetStaticMesh _staticmesh (Variables|/Script/Engine.StaticMeshComponent|GetStaticMesh (Variables|/Game/LevelsParameters/Storing/BP_SelectFood.BP_SelectFood_C|GetStaticMesh (Variables|/Game/LevelsParameters/Storing/StoringPawn.StoringPawn_C|GetFoodRef (Variables|Default|GetPawnRef)))))
          (Rendering|Material|SetMaterial _staticmesh 0 (Rendering|Material|GetMaterial (Variables|/Script/Engine.StaticMeshComponent|GetStaticMesh (Variables|/Game/LevelsParameters/Storing/BP_SelectFood.BP_SelectFood_C|GetStaticMesh (Variables|/Game/LevelsParameters/Storing/StoringPawn.StoringPawn_C|GetFoodRef (Variables|Default|GetPawnRef)))) 0)))
        (:CastFailed
          (Development|PrintString "you trolling you have no storing pawn"))))))

(event Collision|EventActorBeginOverlap
  (params (OtherActor :type Actor%20Object%20Reference)))

(event EventTick
  (params (DeltaSeconds :type Float%20%28single-precision%29)))

(fn ConstructionScript)

(fn SpawnonShelf
  (params (ZTransform :type Float%20%28double-precision%29) (YTransform :type Float%20%28double-precision%29))
  (bind _returnvalue (- ZTransform 23.0))
  (bind _returnvalue_2 (Math|Transform|MakeTransform (Math|Vector|MakeVector 927.0 YTransform _returnvalue) "0, 0, 0" "2.000000,2.000000,2.000000"))
  (Transformation|SetActorTransform (Math|Transform|MakeTransform (.location _returnvalue_2) "0, 0, 0" (.scale _returnvalue_2))))

(fn ZAxisAdjustment
  (switch int (Variables|Default|GetLocationNumber)
    (:1
      ;[1 1 1] Pantry
      (LocalVariables|SetZAdjustment 23.0))
    (:2
      ;[1 1 1] Fridge
      (LocalVariables|SetZAdjustment 23.0))
    (:3
      ;[1 1 1] Freezer
      (LocalVariables|SetZAdjustment 23.0)))
  (return (LocalVariables|GetZAdjustment)))