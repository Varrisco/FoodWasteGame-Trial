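; BP_Trophy is a touchable trophy actor that opens a description widget for the trophy it represents.
; The construction script looks up the actor's display name in TrophiesMap and applies the matching static mesh to Cube.
; A touch on Cube while it is visible adds a WBP_TrophyDescription to the viewport, passing that same display name as TrophyName.
; The display name thus serves as the trophy's identifier for both mesh and description.
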(event OnInputTouchBegin(Cube)
  (params (FingerIndex :type ETouchIndex%20Enum :default "Touch1") (TouchedComponent :type Primitive%20Component%20Object%20Reference))
  (if (Variables|/Script/Engine.SceneComponent|GetbVisible (Variables|Default|GetCube))
    (bind _returnvalue (UserInterface|CreateWidget "/Game/UIElements/WBP_TrophyDescription.WBP_TrophyDescription_C"))
    (Variables|/Game/UIElements/WBP_TrophyDescription.WBP_TrophyDescription_C|SetTrophyName _returnvalue (Utilities|String|StringToName (Utilities|GetDisplayName self)))
    (UserInterface|Viewport|AddtoViewport _returnvalue 0)))

(event EventBeginPlay)

(event Collision|EventActorBeginOverlap
  (params (OtherActor :type Actor%20Object%20Reference)))

(event EventTick
  (params (DeltaSeconds :type Float%20%28single-precision%29)))

(fn ConstructionScript
  (Components|StaticMesh|SetStaticMesh (Variables|Default|GetCube) (.Value (Utilities|Map|Find (Variables|Default|GetTrophiesMap) (Utilities|GetDisplayName self)))))