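; BP_BadFood is a touchable spoiled-food pickup that gets sent to composting.
; Its construction script applies the Mesh variable to the Cube component.
; Touching the Cube plays a sound, calls AddComposting on the game instance and on the first BP_Composting actor found, passing the latter Apple_Quarter, then destroys the food.
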(event OnInputTouchBegin(Cube)
  (params (FingerIndex :type ETouchIndex%20Enum :default "Touch1") (TouchedComponent :type Primitive%20Component%20Object%20Reference))
  (Audio|PlaySound2D "/Game/LevelsParameters/InteractFood.InteractFood" 1.0 1.0 0.0 0 0)
  (bind _asbp_main_game_instance (CallFunction|GetGameInstance))
  (Default|AddComposting _asbp_main_game_instance)
  (bind _outactors (Actor|GetAllActorsOfClass "/Game/LevelsParameters/MainLevel/BP_Composting.BP_Composting_C"))
  (Default|AddComposting (Utilities|Array|Get(acopy) _outactors) "/Game/LevelsParameters/MeshesAndMaterials/Slices/Apple_Quarter.Apple_Quarter")
  (Actor|DestroyActor))

(event EventBeginPlay)

(event Collision|EventActorBeginOverlap
  (params (OtherActor :type Actor%20Object%20Reference)))

(event EventTick
  (params (DeltaSeconds :type Float%20%28single-precision%29)))

(fn ConstructionScript
  (Components|StaticMesh|SetStaticMesh (Variables|Default|GetCube) (Variables|Default|GetMesh)))