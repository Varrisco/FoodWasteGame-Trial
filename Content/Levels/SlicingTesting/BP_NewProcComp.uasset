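; Test actor for runtime mesh slicing that turns a configurable static mesh into a sliceable procedural mesh.
; The construction script copies the static mesh into a procedural mesh with collision, then destroys the source component.
; SliceMe cuts the given component along a plane up to four times, capping cuts with a tomato material.
; Each slice's output gets physics and a custom collision channel, then a radial impulse fires at the cut.
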(event Custom|SliceMe
  (params (Proc%20Comp :type Procedural%20Mesh%20Component%20Object%20Reference) (Location :type Vector) (Normal :type Vector))
  (bind _radialforce (Variables|Default|GetRadialForce))
  (Utilities|FlowControl|DoN 4 ; This would be useful to cut only N times.
    (:Exit
      (bind _outotherhalfprocmesh (Class|KismetProceduralMeshLibrary|SliceProceduralMesh Proc%20Comp Location Normal false "CreateNewSectionForCap" "/Game/GameAssets/Materials/M_Tomato.M_Tomato"))
      (Physics|SetSimulatePhysics _outotherhalfprocmesh true)
      (Collision|SetCollisionObjectType _outotherhalfprocmesh "ECC_GameTraceChannel1")
      (Transformation|SetWorldLocation _radialforce Location false true)
      (Class|RadialForceComponent|FireImpulse _radialforce))))

(event EventBeginPlay)

(event Collision|EventActorBeginOverlap
  (params (OtherActor :type Actor%20Object%20Reference)))

(event EventTick
  (params (DeltaSeconds :type Float%20%28single-precision%29)))

(fn ConstructionScript
  (Components|StaticMesh|SetStaticMesh (Variables|Default|GetStaticMesh) (Variables|Default|GetStaticMeshToCopy))
  (Class|KismetProceduralMeshLibrary|CopyProceduralMeshfromStaticMeshComponent (Variables|Default|GetStaticMesh) 0 (Variables|Default|GetProceduralMesh) true)
  (Components|DestroyComponent (Variables|Default|GetStaticMesh)))