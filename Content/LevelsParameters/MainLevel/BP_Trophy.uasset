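; BP_Trophy is a touchable trophy actor that shows whether it is earned and opens its description.
; Its display name is the key for the construction-script mesh, the widget's trophy name and the GameInstance earned check.
; UnlockTrophy clears the locked overlay for earned trophies but is not called within this Blueprint.
; Touch resets all trophies' overlays, removes open description widgets, then highlights this trophy blue with a new widget.
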(event OnInputTouchBegin(Cube)
  (params (FingerIndex :type ETouchIndex%20Enum :default "Touch1") (TouchedComponent :type Primitive%20Component%20Object%20Reference))
  (CallFunction|ClearHighlightandWdiget)
  (bind _returnvalue (UserInterface|CreateWidget "/Game/UIElements/WBP_TrophyDescription.WBP_TrophyDescription_C"))
  (Variables|/Game/UIElements/WBP_TrophyDescription.WBP_TrophyDescription_C|SetTrophyName _returnvalue (Utilities|String|StringToName (Utilities|GetDisplayName self)))
  (UserInterface|Viewport|AddtoViewport _returnvalue 0)
  (Rendering|Material|SetOverlayMaterial (Variables|Default|GetCube) "/Game/LevelsParameters/MainLevel/MI_BlueOverlay.MI_BlueOverlay" :!class /Script/Engine.MeshComponent))

(event EventBeginPlay)

(event Collision|EventActorBeginOverlap
  (params (OtherActor :type Actor%20Object%20Reference)))

(event EventTick
  (params (DeltaSeconds :type Float%20%28single-precision%29)))

(fn ConstructionScript
  (bind _cube (Variables|Default|GetCube))
  (Components|StaticMesh|SetStaticMesh (Variables|Default|GetCube) (.Value (Utilities|Map|Find (Variables|Default|GetTrophiesMap) (Utilities|GetDisplayName self))))
  (if (Variables|Default|GetUnlocked)
    (Rendering|Material|SetOverlayMaterial _cube 0 :!class /Script/Engine.MeshComponent)
    (else
      (Rendering|Material|SetOverlayMaterial _cube "/Game/LevelsParameters/Customization/MeshesAndMaterials/MI_NotUnlocked.MI_NotUnlocked" :!class /Script/Engine.MeshComponent))))

(fn UnlockTrophy
  (bind _asbp_main_game_instance (CallFunction|GetGameInstance))
  (if (Utilities|Array|ContainsItem (Variables|/Game/TopDown/Blueprints/BP_MainGameInstance.BP_MainGameInstance_C|GetTrophiesEarned _asbp_main_game_instance) (Utilities|GetDisplayName self))
    (Variables|Default|SetUnlocked true)
    (Rendering|Material|SetOverlayMaterial (Variables|Default|GetCube) 0 :!class /Script/Engine.MeshComponent)))

(fn ClearHighlightandWdiget
  (bind _outactors (Actor|GetAllActorsOfClass "BP_Trophy_C"))
  (for _array_element _outactors
    (if (Variables|BP_Trophy_C|GetUnlocked _array_element)
      (Rendering|Material|SetOverlayMaterial (Variables|BP_Trophy_C|GetCube _array_element) 0 :!class /Script/Engine.MeshComponent)
      (else
        (Rendering|Material|SetOverlayMaterial (Variables|BP_Trophy_C|GetCube _array_element) "/Game/LevelsParameters/Customization/MeshesAndMaterials/MI_NotUnlocked.MI_NotUnlocked" :!class /Script/Engine.MeshComponent))))
  (bind _foundwidgets (Widget|GetAllWidgetsOfClass "/Game/UIElements/WBP_TrophyDescription.WBP_TrophyDescription_C" true))
  (for _array_element_2 _foundwidgets
    (Widget|RemovefromParent _array_element_2))
  (return))