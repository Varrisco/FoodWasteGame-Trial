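; BP_SelectFood is a touch-selectable food item in the food storing level, with its mesh taken from FoodData at construction.
; On touch, it registers itself and its mesh with the StoringPawn, cached on BeginPlay.
; ThrowFood enables physics and applies an impulse picked by the storing zone's display name to launch it toward that fridge, pantry or freezer shelf or fridge door.
; A separate function switches physics off.
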(event OnInputTouchBegin(StaticMesh)
  (params (FingerIndex :type ETouchIndex%20Enum :default "Touch1") (TouchedComponent :type Primitive%20Component%20Object%20Reference))
  (bind _pawnref (Variables|Default|GetPawnRef))
  (Default|SetFoodRef _pawnref self)
  (Default|ChangeFoodMesh(Changed) _pawnref (Variables|/Script/Engine.StaticMeshComponent|GetStaticMesh (Variables|Default|GetStaticMesh))))

(event EventBeginPlay
  ;[1 1 1] Getting a reference to storingPawn to avoid recasts
  (Utilities|IsValid (Variables|Default|GetPawnRef)
    (:Is%20Not%20Valid
      (bind _asstoring_pawn (Utilities|Casting|CastToStoringPawn (Game|Player|GetPlayerPawn 0))
        (:then
          (Variables|Default|SetPawnRef _asstoring_pawn))
        (:CastFailed
          (Development|PrintString "you trolling you have no storing pawn"))))))

(event Collision|EventActorBeginOverlap
  (params (OtherActor :type Actor%20Object%20Reference)))

(event EventTick
  (params (DeltaSeconds :type Float%20%28single-precision%29)))

(fn ConstructionScript
  (Components|StaticMesh|SetStaticMesh (Variables|Default|GetStaticMesh) (Variables|/Game/LevelsParameters/Storing/Structures/FoodDataAsset.FoodDataAsset_C|GetMesh (Variables|Default|GetFoodData))))

(fn SpawnonShelfUNUSED
  (params (FoodRef :type BP%20Select%20Food%20Object%20Reference) (ZTransform :type Float%20%28double-precision%29) (YTransform :type Float%20%28double-precision%29))
  (if (Utilities|Enum|Equal(Enum) (Utilities|GetObjectName FoodRef) (Utilities|GetObjectName self))
    (Transformation|SetActorTransform (Math|Transform|MakeTransform (Math|Vector|MakeVector 954.927979 YTransform ZTransform)))))

(fn ThrowFood
  (params (StoringZone :type BP%20Storing%20Zone%20Object%20Reference))
  (bind _staticmesh (Variables|Default|GetStaticMesh))
  (Physics|SetSimulatePhysics _staticmesh true)
  (switch string (Utilities|GetDisplayName StoringZone)
    (:FridgeShelf1
      ;[1 1 1] Fridge Shelf 1 & Pantry Shelf 1
      (Physics|AddImpulse _staticmesh "300.000000,0.000000,200.000000" "None" false :!label _label))
    (:PantryShelf1
      (goto _label))
    (:FridgeShelf2
      ;[1 1 1] Fridge Shelf 2 & Freezer 1
      (Physics|AddImpulse _staticmesh "300.000000,0.000000,130.000000" "None" false :!label _label_2))
    (:PantryShelf2
      ;[1 1 1] Fridge Shelf 3 & Pantry Shelf 2 & Freezer 2
      (Physics|AddImpulse _staticmesh "300.000000,0.000000,50.000000" "None" false :!label _label_3))
    (:FridgeShelf3
      (goto _label_3))
    (:PantryShelf3
      ;[1 1 1] Fridge Shelf 4 & Pantry Shelf 3 & Freezer 3
      (Physics|AddImpulse _staticmesh "300.000000,0.000000,-50.000000" "None" false :!label _label_4))
    (:FridgeShelf4
      (goto _label_4))
    (:FreezerShelf1
      (goto _label_2))
    (:FreezerShelf2
      (goto _label_3))
    (:FreezerShelf3
      (goto _label_4))
    (:FridgeDoor
      ;[1 1 1] Fridge Left door
      (Physics|AddImpulse _staticmesh "300.000000,-180.000000,0.000000" "None" false))))

(fn DisableSimulatePhysics
  (Physics|SetSimulatePhysics (Variables|Default|GetStaticMesh) false))