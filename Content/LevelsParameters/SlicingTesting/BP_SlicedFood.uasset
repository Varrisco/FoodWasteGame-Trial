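; BP_SlicedFood is a sliced food piece actor for the slicing game that reacts to touch.
; Its construction script applies the configured mesh, then a bad-food material, or a yellow material for good butter.
; On BeginPlay, an unset pawn reference is filled from the player's SliceGamePawn, which has slicing disabled and is swept to a fixed Y.
; Touching the mesh moves the actor to a hardcoded location, then enables physics after a short delay.
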(event OnInputTouchBegin(StaticMesh)
  (params (FingerIndex :type ETouchIndex%20Enum :default "Touch1") (TouchedComponent :type Primitive%20Component%20Object%20Reference))
  (Transformation|SetActorLocation "986.226500,212.681345,137.861993" false false)
  (Utilities|FlowControl|Delay 0.1)
  (Physics|SetSimulatePhysics (Variables|Default|GetStaticMesh) true))

(event EventBeginPlay
  (Utilities|IsValid (Variables|Default|GetPawnRef)
    (:Is%20Not%20Valid
      (bind _asslice_game_pawn (Utilities|Casting|CastToSliceGamePawn (Game|Player|GetPlayerPawn 0))
        (:then
          (Variables|Default|SetPawnRef _asslice_game_pawn)
          (Default|DisableSlicing (Variables|Default|GetPawnRef))
          (Transformation|SetActorLocation (Variables|Default|GetPawnRef) (Math|Vector|MakeVector (.x (Transformation|GetActorLocation (Variables|Default|GetPawnRef))) 37.785679 (.z (Transformation|GetActorLocation (Variables|Default|GetPawnRef)))) true false))
        (:CastFailed
          (Development|PrintString "you trolling you have no slicing  pawn"))))))

(event Collision|EventActorBeginOverlap
  (params (OtherActor :type Actor%20Object%20Reference)))

(event EventTick
  (params (DeltaSeconds :type Float%20%28single-precision%29)))

(fn ConstructionScript
  (bind _staticmesh (Variables|Default|GetStaticMesh))
  (Components|StaticMesh|SetStaticMesh (Variables|Default|GetStaticMesh) (Variables|Default|GetSliceMeshToSet))
  (if (Variables|Default|GetisBadFood)
    (Rendering|Material|SetMaterial _staticmesh 0 "/Game/LevelsParameters/SlicingTesting/UnrealExample/M_BadFood.M_BadFood")
    (elif (== (Variables|Default|GetFoodName) "Butter")
      (Rendering|Material|SetMaterial _staticmesh 0 "/Game/LevelsParameters/MeshesAndMaterials/MaterialsTextures/YellowGoodButter.YellowGoodButter"))))