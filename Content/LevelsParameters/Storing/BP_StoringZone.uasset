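; Storage zone actor for the food-storing level, representing a named pantry, fridge or freezer spot.
; Box overlap registers it as the StoringPawn's current zone, localizes the BP_StoringArrow text materials and toggles an outline.
; DefineMaterial checks selected food against the zone's StoringDataTable row, switching the tutorial highlight and green or red outline.
; Store functions spawn BP_StoredFood at hard-coded shelf or door slots indexed by remaining Capacity, then decrement it.
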(event OnComponentBeginOverlap(StoringBoxCollision)
  (params (OverlappedComponent :type Primitive%20Component%20Object%20Reference) (OtherActor :type Actor%20Object%20Reference) (OtherComp :type Primitive%20Component%20Object%20Reference) (OtherBodyIndex :type Integer) (bFromSweep :type Boolean) (SweepResult :type Hit%20Result%20Structure%20%28by%20ref%29))
  (Variables|Default|SetArrowInZone true)
  (Variables|/Game/LevelsParameters/Storing/StoringPawn.StoringPawn_C|SetCurrentZoneRef (Variables|Default|GetPawnRef) self)
  (bind _returnvalue (Actor|GetActorOfClass "/Game/LevelsParameters/Storing/BP_StoringArrow.BP_StoringArrow_C"))
  (bind _asbp_main_game_instance (CallFunction|GetGameInstance))
  (switch string (Variables|/Game/TopDown/Blueprints/BP_MainGameInstance.BP_MainGameInstance_C|GetLanguage _asbp_main_game_instance)
    (:en
      (Default|SetArrowText&Material _returnvalue (Variables|Default|GetZoneArrowTextEN) (Variables|Default|GetZoneTemperatureTextEN)))
    (:pt
      (Default|SetArrowText&Material _returnvalue (Variables|Default|GetZoneArrowText) (Variables|Default|GetZoneTemperatureText))))
  (Development|SetHiddeninGame (Variables|Default|GetCurrentBoxOutline) false false))

(event OnComponentEndOverlap(StoringBoxCollision)
  (params (OverlappedComponent :type Primitive%20Component%20Object%20Reference) (OtherActor :type Actor%20Object%20Reference) (OtherComp :type Primitive%20Component%20Object%20Reference) (OtherBodyIndex :type Integer))
  (Variables|Default|SetArrowInZone false)
  (Development|SetHiddeninGame (Variables|Default|GetCurrentBoxOutline) true false))

(event EventBeginPlay
  ;[1 1 1] Getting a reference to storingPawn to avoid recasts
  (Utilities|IsValid (Variables|Default|GetPawnRef)
    (:Is%20Not%20Valid
      (bind _asstoring_pawn (Utilities|Casting|CastToStoringPawn (Game|Player|GetPlayerPawn 0))
        (:then
          (Variables|Default|SetPawnRef _asstoring_pawn)
          (CallFunction|SetLocationNumber)
          (Variables|Default|SetCurrentBoxOutline (Variables|Default|GetStoringBoxOutlineRed)))
        (:CastFailed
          (Development|PrintString "you trolling you have no storing pawn"))))))

(event Collision|EventActorBeginOverlap
  (params (OtherActor :type Actor%20Object%20Reference)))

(event EventTick
  (params (DeltaSeconds :type Float%20%28single-precision%29)))

(fn ConstructionScript)

(fn StoreFoodwithSlots
  (params (StoredZone :type BP%20Storing%20Zone%20Object%20Reference))
  (if (not (== (Variables|Default|GetCapacity) 0))
    (switch int (Variables|Default|GetLocationNumber)
      (:1
        (bind _ytransform (CallFunction|StorePantryShelves (Variables|Default|GetCapacity)))
        (LocalVariables|SetYTransform _ytransform))
      (:2
        (bind _ytransform_2 (CallFunction|StoreFFShelves (Variables|Default|GetCapacity)))
        (LocalVariables|SetYTransform _ytransform_2))
      (:3
        (bind _ytransform_3 (CallFunction|StoreFFShelves (Variables|Default|GetCapacity)))
        (LocalVariables|SetYTransform _ytransform_3)))
    (bind _returnvalue (Game|SpawnActorfromClass "/Game/LevelsParameters/Storing/BP_StoredFood.BP_StoredFood_C" (Math|Transform|MakeTransform "0, 0, 0" "0, 0, 0" "1.000000,1.000000,1.000000") "Undefined" 0 0 StoredZone 0))
    (Default|SpawnonShelf _returnvalue (.z (Transformation|GetActorLocation)) (LocalVariables|GetYTransform))
    (bind _result (Math|Integer|DecrementInt (Variables|Default|GetCapacity))
      (:%20%20
        (Variables|Default|SetCapacity _result)
        (return _returnvalue)))))

(fn StoreFoodDoorswithSlots
  (params (StoringZone :type BP%20Storing%20Zone%20Object%20Reference))
  (bind _ztransform (CallFunction|StoreDoorShelves (Variables|Default|GetCapacity)))
  (LocalVariables|SetZTransform _ztransform)
  (bind _returnvalue (Game|SpawnActorfromClass "/Game/LevelsParameters/Storing/BP_StoredFood.BP_StoredFood_C" (Math|Transform|MakeTransform "0, 0, 0" "0, 0, 0" "1.000000,1.000000,1.000000") "Undefined" 0 0 StoringZone 0))
  (Default|SpawnonShelf _returnvalue (LocalVariables|GetZTransform) -158.548499)
  (bind _result (Math|Integer|DecrementInt (Variables|Default|GetCapacity))
    (:%20%20
      (Variables|Default|SetCapacity _result))))

(fn StorePantryShelves
  (params (Capacity :type Integer))
  (switch int Capacity
    (:0
      (Development|PrintString "A prateleira está cheia"))
    (:1
      (LocalVariables|SetYTransformF -462.729736)
      (return (LocalVariables|GetYTransformF)))
    (:2
      (LocalVariables|SetYTransformF -508.729736)
      (return (LocalVariables|GetYTransformF)))
    (:3
      (LocalVariables|SetYTransformF -554.729736)
      (return (LocalVariables|GetYTransformF)))
    (:4
      (LocalVariables|SetYTransformF -603.729736)
      (return (LocalVariables|GetYTransformF)))))

(fn StoreFFShelves
  (params (Capacity :type Integer))
  (switch int Capacity
    (:0
      (Development|PrintString "A prateleira está cheia"))
    (:1
      (LocalVariables|SetYTransformF 63.0)
      (return (LocalVariables|GetYTransformF)))
    (:2
      (LocalVariables|SetYTransformF 2e+01)
      (return (LocalVariables|GetYTransformF)))
    (:3
      (LocalVariables|SetYTransformF -25.0)
      (return (LocalVariables|GetYTransformF)))
    (:4
      (LocalVariables|SetYTransformF -7e+01)
      (return (LocalVariables|GetYTransformF)))))

(fn StoreDoorShelves
  (params (Capacity :type Integer))
  (switch int Capacity
    (:0
      (Development|PrintString "A prateleira está cheia"))
    (:1
      (LocalVariables|SetZTransformF 257.0)
      (return (LocalVariables|GetZTransformF)))
    (:2
      (LocalVariables|SetZTransformF 352.0)
      (return (LocalVariables|GetZTransformF)))
    (:3
      (LocalVariables|SetZTransformF 435.237598)
      (return (LocalVariables|GetZTransformF)))))

(fn SetGoodMaterial
  (bind _tutorialzonecolor (Variables|Default|GetTutorialZoneColor))
  (if (Utilities|Enum|Equal(Enum) (Variables|Default|GetName self) "FridgeDoor")
    (Rendering|Material|SetMaterial _tutorialzonecolor 0 "/Game/LevelsParameters/Storing/ColorsMaterial/MI_SolidGreen.MI_SolidGreen")
    (Development|SetHiddeninGame _tutorialzonecolor false true)
    (Rendering|SetVisibility _tutorialzonecolor true true)
    (Variables|Default|SetCurrentBoxOutline (Variables|Default|GetStoringBoxOutlineGreen))
    (else
      (Rendering|Material|SetMaterial _tutorialzonecolor 0 "/Game/LevelsParameters/Storing/ColorsMaterial/MI_GreenOverlay.MI_GreenOverlay")
      (Development|SetHiddeninGame _tutorialzonecolor false true)
      (Variables|Default|SetCurrentBoxOutline (Variables|Default|GetStoringBoxOutlineGreen)))))

(fn SetBadMaterial
  (bind _tutorialzonecolor (Variables|Default|GetTutorialZoneColor))
  (Rendering|Material|SetMaterial _tutorialzonecolor 0 "/Game/LevelsParameters/Storing/ColorsMaterial/MI_SolidYellow.MI_SolidYellow")
  (Development|SetHiddeninGame _tutorialzonecolor true false)
  (Rendering|SetVisibility _tutorialzonecolor false true)
  (Variables|Default|SetCurrentBoxOutline (Variables|Default|GetStoringBoxOutlineRed)))

(fn DefineMaterial
  (params (SelectedFoodRef :type BP%20Select%20Food%20Object%20Reference))
  (bind _returnvalue (Utilities|GetDataTableRow "/Game/LevelsParameters/Storing/Structures/StoringDataTable.StoringDataTable" (Utilities|String|StringToName (Variables|Default|GetName self)))
    (:then
      (bind _foodcomp (CallFunction|CheckCompFood (.CompatibleFood (Utilities|Struct|BreakStoringStruct _returnvalue)) SelectedFoodRef))
      (if _foodcomp
        (CallFunction|SetGoodMaterial)
        (else
          (CallFunction|SetBadMaterial))))))

(fn CheckCompFood
  (params (DTZoneFoodArray :type Array%20of%20Food%20Data%20Asset%20Object%20References) (Food :type BP%20Select%20Food%20Object%20Reference))
  (for _array_element DTZoneFoodArray
    (if (== _array_element (Variables|/Game/LevelsParameters/Storing/BP_SelectFood.BP_SelectFood_C|GetFoodData Food))
      ;[1 1 1] Found
      (return (== _array_element (Variables|/Game/LevelsParameters/Storing/BP_SelectFood.BP_SelectFood_C|GetFoodData Food)))))
  ;[1 1 1] Not Found
  (return (== _array_element (Variables|/Game/LevelsParameters/Storing/BP_SelectFood.BP_SelectFood_C|GetFoodData Food))))

(fn SetLocationNumber
  (bind _self self)
  (bind _name (Variables|Default|GetName _self))
  ;[1 1 1] 1 Pantry 2 Fridge 3 Freezer
  (if (Utilities|String|Contains _name "Freezer")
    (Variables|Default|SetLocationNumber 3)
    (elif (Utilities|String|Contains _name "Fridge")
      (Variables|Default|SetLocationNumber 2)
      (elif (Utilities|String|Contains _name "Pantry")
        (Variables|Default|SetLocationNumber 1)))))