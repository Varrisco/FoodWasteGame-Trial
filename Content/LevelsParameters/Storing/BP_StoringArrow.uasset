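; BP_StoringArrow is an arrow actor that bobs vertically between a minimum and maximum height.
; BeginPlay starts a looping 0.01-second timer instead of using Tick, intended to keep movement framerate independent.
; Each timer call runs ArrowMovementUpAndDown, which shifts Z by MovementSpeed and flips IsGoingUp at either limit.
; An alternative ArrowMovementUpThenReset function exists but is never called.
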(event Custom|CheckMovement
  (Utilities|Time|SetTimerbyEvent (delegate Custom|Move) 0.01 true))

(event Custom|Move
  (CallFunction|ArrowMovementUpandDown) ; This one moves the arrow up and down
)

(event EventBeginPlay
  ;[1 1 1] Way to make it framerate independent (along with the custom events
  (CallFunction|CheckMovement))

(event Collision|EventActorBeginOverlap
  (params (OtherActor :type Actor%20Object%20Reference)))

(event EventTick
  (params (DeltaSeconds :type Float%20%28single-precision%29)))

(fn ConstructionScript)

(fn ArrowMovementUpThenReset
  (bind _returnvalue (Transformation|GetActorLocation))
  (bind _movementspeed (Variables|Default|GetMovementSpeed))
  (Development|PrintString (Utilities|String|Append "x " (Utilities|String|ToString(Float) (.x _returnvalue)) " y " (Utilities|String|ToString(Float) (.y _returnvalue)) " z " (Utilities|String|ToString(Float) (.z _returnvalue))))
  (if (>= (.z _returnvalue) (Variables|Default|GetZMaxValue))
    (Transformation|SetActorRelativeLocation (Math|Vector|MakeVector (.x _returnvalue) (.y _returnvalue) (- (.z _returnvalue) _movementspeed)) :!label _label)
    (if (<= (.z _returnvalue) (Variables|Default|GetZMinValue))
      _
      (else
        (goto _label))))
  (Transformation|SetActorRelativeLocation (Math|Vector|MakeVector (.x _returnvalue) (.y _returnvalue) (+ (.z _returnvalue) _movementspeed))))

(fn ArrowMovementUpandDown
  (bind _returnvalue (Transformation|GetActorLocation))
  (bind _movementspeed (Variables|Default|GetMovementSpeed))
  (if (Variables|Default|GetisGoingUp)
    (if (>= (.z _returnvalue) (Variables|Default|GetZMaxValue))
      (Variables|Default|SetisGoingUp false)
      (else
        (Transformation|SetActorRelativeLocation (Math|Vector|MakeVector (.x _returnvalue) (.y _returnvalue) (+ (.z _returnvalue) _movementspeed)))))
    (elif (<= (.z _returnvalue) (Variables|Default|GetZMinValue))
      (Variables|Default|SetisGoingUp true)
      (else
        (Transformation|SetActorRelativeLocation (Math|Vector|MakeVector (.x _returnvalue) (.y _returnvalue) (- (.z _returnvalue) _movementspeed)))))))