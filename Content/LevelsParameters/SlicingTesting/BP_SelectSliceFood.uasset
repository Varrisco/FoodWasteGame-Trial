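; Selectable food pickup for the slicing stage, showing its data asset's mesh with good or bad material variants, with Butter handled separately.
; On touch it moves the slicing pawn to the cutting position, flags the controller and spawns a BP_NewProcComp from the food data.
; It also hands the food to the pawn, registers itself for slice scoring, and updates recipe text in the UI and a world text actor.
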(event OnInputTouchBegin(StaticMesh)
  (params (FingerIndex :type ETouchIndex%20Enum :default "Touch1") (TouchedComponent :type Primitive%20Component%20Object%20Reference))
  (bind _pawnref (Variables|Default|GetPawnRef))
  (Audio|PlaySound2D "/Game/LevelsParameters/InteractFood2.InteractFood2" 1.0 1.0 0.0 0 0)
  (CallFunction|MovetoSlicePosition)
  (CallFunction|SpawnProcFood)
  (Variables|/Game/LevelsParameters/SlicingTesting/UnrealExample/SliceGamePawn.SliceGamePawn_C|SetFoodRef _pawnref (Variables|Default|GetSliceFoodDataAsset))
  (Default|SetSlicedFoodScore (Variables|/Game/LevelsParameters/SlicingTesting/UnrealExample/SliceGamePawn.SliceGamePawn_C|GetSlicingManager _pawnref) self))

(event EventBeginPlay
  (Utilities|IsValid (Variables|Default|GetPawnRef)
    (:Is%20Not%20Valid
      (bind _asslice_game_pawn (CallFunction|GetSlicingPawn))
      (Variables|Default|SetPawnRef _asslice_game_pawn)
      (bind _asslice_game_player_controller (Utilities|Casting|CastToSliceGamePlayerController (Game|GetPlayerController 0)))
      (Variables|Default|SetPControllerRef _asslice_game_player_controller)
      (Components|StaticMesh|SetStaticMesh (Variables|Default|GetStaticMesh) (Variables|/Game/LevelsParameters/SlicingTesting/Structures/SliceFoodDataAsset.SliceFoodDataAsset_C|GetMainMesh (Variables|Default|GetSliceFoodDataAsset))))))

(event Collision|EventActorBeginOverlap
  (params (OtherActor :type Actor%20Object%20Reference)))

(event EventTick
  (params (DeltaSeconds :type Float%20%28single-precision%29)))

(fn ConstructionScript
  (bind _staticmesh (Variables|Default|GetStaticMesh))
  (bind _staticmesh_2 (Variables|Default|GetStaticMesh))
  (if (== (Variables|/Game/LevelsParameters/SlicingTesting/Structures/SliceFoodDataAsset.SliceFoodDataAsset_C|GetName (Variables|Default|GetSliceFoodDataAsset)) "Butter")
    (if (Variables|Default|GetisBadFood)
      (Rendering|Material|SetMaterial _staticmesh 1 "/Game/LevelsParameters/MeshesAndMaterials/MaterialsTextures/YellowBadButter.YellowBadButter")
      (else
        (Rendering|Material|SetMaterial _staticmesh 1 "/Game/LevelsParameters/MeshesAndMaterials/MaterialsTextures/YellowGoodButter.YellowGoodButter")
        (Rendering|Material|SetMaterial _staticmesh 0 "/Game/LevelsParameters/MeshesAndMaterials/MaterialsTextures/YellowGoodButter.YellowGoodButter")))
    (elif (Variables|Default|GetisBadFood)
      (Rendering|Material|SetMaterial _staticmesh_2 1 "/Game/LevelsParameters/SlicingTesting/UnrealExample/M_BADUniversalFoodMaterial.M_BADUniversalFoodMaterial")
      (else
        (Rendering|Material|SetMaterial _staticmesh_2 1 "/Game/LevelsParameters/MeshesAndMaterials/MaterialsTextures/M_UniversalFoodMaterial.M_UniversalFoodMaterial")))))

(fn MovetoSlicePosition
  (Transformation|SetRelativeLocation (Variables|/Script/Engine.Actor|GetRootComponent (Variables|Default|GetPawnRef)) "755.250257,-12.604689,175.117329" false false)
  (Variables|/Game/LevelsParameters/SlicingTesting/UnrealExample/SliceGamePlayerController.SliceGamePlayerController_C|SetIsCuttingArea (Variables|Default|GetPControllerRef) true))

(fn SpawnProcFood
  (bind _pawnref (Variables|Default|GetPawnRef))
  (bind _slicefooddataasset (Variables|Default|GetSliceFoodDataAsset))
  (bind _transformscalemultiply (Variables|/Game/LevelsParameters/SlicingTesting/Structures/SliceFoodDataAsset.SliceFoodDataAsset_C|GetTransformScaleMultiply _slicefooddataasset))
  (bind _cookingmanager (Variables|/Game/LevelsParameters/SlicingTesting/UnrealExample/SliceGamePawn.SliceGamePawn_C|GetCookingManager _pawnref))
  (bind _activecookingfood (Variables|/Game/LevelsParameters/Cooking/Structures/Cooking_Manager.Cooking_Manager_C|GetActiveCookingFood _cookingmanager))
  (bind _recipeinstructions (Variables|/Game/LevelsParameters/Cooking/Structures/RecipeDataAsset.RecipeDataAsset_C|GetRecipeInstructions _activecookingfood))
  (bind _output (Utilities|Array|Get(acopy) _recipeinstructions 4))
  (bind _returnvalue (Utilities|String|ToString(Text) _output))
  (bind (_lefts _rights) (Utilities|String|Split _returnvalue "("))
  (Game|SpawnActorfromClass "/Game/LevelsParameters/SlicingTesting/BP_NewProcComp.BP_NewProcComp_C" (Math|Transform|MakeTransform "929.884911,-15.831220,114.126350" "0, 0, 0" (Math|Vector|MakeVector _transformscalemultiply _transformscalemultiply _transformscalemultiply)) "Undefined" 0 _slicefooddataasset (Variables|Default|GetisBadFood) 0)
  (bind _foundwidgets (Widget|GetAllWidgetsOfClass "/Game/UIElements/WBP_CommonUI.WBP_CommonUI_C" true))
  (Variables|/Game/UIElements/WBP_CommonUI.WBP_CommonUI_C|SetRecipeString (Utilities|Array|Get(acopy) _foundwidgets) (Utilities|String|ToString(Text) _output))
  (bind _outactors (Actor|GetAllActorsOfClass "/Script/Engine.TextRenderActor"))
  (Rendering|Components|TextRender|SetText (Variables|/Script/Engine.TextRenderActor|GetTextRender (Utilities|Array|Get(acopy) _outactors)) (Utilities|Text|FormatText "{left}
({right} " _lefts _rights)))