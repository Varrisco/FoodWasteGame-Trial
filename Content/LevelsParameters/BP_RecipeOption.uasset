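; Touchable food actor representing a recipe choice, with its mesh pulled from the game instance's food data by index at construction.
; On touch, it removes that food and expiry entry from BP_MainGameInstance, stores its recipe as active, and swaps the recipe widget for first-step instructions and dialogue in the common UI.
; It then unhides the slicing level-change zone, found by display name, and destroys every recipe option actor.
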(event OnInputTouchBegin(Cube)
  (params (FingerIndex :type ETouchIndex%20Enum :default "Touch1") (TouchedComponent :type Primitive%20Component%20Object%20Reference))
  (bind _foundwidgets (Widget|GetAllWidgetsOfClass "/Game/UIElements/WBP_CommonUI.WBP_CommonUI_C" true))
  (Widget|SetVisibility (Variables|/Game/UIElements/WBP_CommonUI.WBP_CommonUI_C|GetRecipeBox (Utilities|Array|Get(acopy) _foundwidgets)) "Visible")
  (Variables|/Game/UIElements/WBP_CommonUI.WBP_CommonUI_C|SetDialogueString (Utilities|Array|Get(acopy) _foundwidgets) "Agora segue as instruções da receita no canto inferior esquerdo.")
  (Variables|/Game/UIElements/WBP_CommonUI.WBP_CommonUI_C|SetRecipeString (Utilities|Array|Get(acopy) _foundwidgets) (Utilities|Array|Get(acopy) (Variables|/Game/LevelsParameters/Cooking/Structures/RecipeDataAsset.RecipeDataAsset_C|GetRecipeInstructions (Variables|Default|GetRecipe))))
  (bind _foundwidgets_2 (Widget|GetAllWidgetsOfClass "/Game/UIElements/WBP_Recipe.WBP_Recipe_C" true))
  (Widget|RemovefromParent (Utilities|Array|Get(acopy) _foundwidgets_2))
  (bind _asbp_main_game_instance (CallFunction|RemoveFoodGameInstance))
  (Variables|/Game/TopDown/Blueprints/BP_MainGameInstance.BP_MainGameInstance_C|SetActiveRecipe _asbp_main_game_instance (Variables|Default|GetRecipe))
  (bind _asbp_main_game_instance_2 (Utilities|Casting|CastToBP_MainGameInstance (Game|GetGameInstance)))
  (Development|PrintString (Utilities|String|ToString(Name) (Variables|/Game/LevelsParameters/Cooking/Structures/RecipeDataAsset.RecipeDataAsset_C|GetName (Variables|/Game/TopDown/Blueprints/BP_MainGameInstance.BP_MainGameInstance_C|GetActiveRecipe _asbp_main_game_instance_2))) true true "(R=0.000000,G=0.660000,B=1.000000,A=1.000000)" 1e+01)
  (CallFunction|EnableSlicingLevel)
  (bind _outactors (Actor|GetAllActorsOfClass "BP_RecipeOption_C"))
  (for _array_element _outactors
    (Actor|DestroyActor _array_element)))

(event EventBeginPlay
  (bind _cube (Variables|Default|GetCube))
  (if (Utilities|Enum|Equal(Enum) (Utilities|GetDisplayName (Variables|/Script/Engine.StaticMeshComponent|GetStaticMesh _cube)) "Butter")
    (Rendering|Material|SetMaterial _cube 0 "/Game/LevelsParameters/MeshesAndMaterials/MaterialsTextures/YellowGoodButter.YellowGoodButter")))

(event Collision|EventActorBeginOverlap
  (params (OtherActor :type Actor%20Object%20Reference)))

(event EventTick
  (params (DeltaSeconds :type Float%20%28single-precision%29)))

(fn ConstructionScript
  (bind _asbp_main_game_instance (Utilities|Casting|CastToBP_MainGameInstance (Game|GetGameInstance)))
  (Components|StaticMesh|SetStaticMesh (Variables|Default|GetCube) (Variables|/Game/LevelsParameters/Storing/Structures/FoodDataAsset.FoodDataAsset_C|GetMesh (Utilities|Array|Get(acopy) (Variables|/Game/TopDown/Blueprints/BP_MainGameInstance.BP_MainGameInstance_C|GetFoodDataElement _asbp_main_game_instance) (Variables|Default|GetGameInstanceIndex)))))

(fn RemoveFoodGameInstance
  (bind _gameinstanceindex (Variables|Default|GetGameInstanceIndex))
  (bind _asbp_main_game_instance (Utilities|Casting|CastToBP_MainGameInstance (Game|GetGameInstance)))
  (Utilities|Array|RemoveItem (Variables|/Game/TopDown/Blueprints/BP_MainGameInstance.BP_MainGameInstance_C|GetFoodDataElement _asbp_main_game_instance) (Utilities|Array|Get(acopy) (Variables|/Game/TopDown/Blueprints/BP_MainGameInstance.BP_MainGameInstance_C|GetFoodDataElement _asbp_main_game_instance) _gameinstanceindex))
  (Utilities|Array|RemoveItem (Variables|/Game/TopDown/Blueprints/BP_MainGameInstance.BP_MainGameInstance_C|GetFoodExpiryElement _asbp_main_game_instance) (Utilities|Array|Get(acopy) (Variables|/Game/TopDown/Blueprints/BP_MainGameInstance.BP_MainGameInstance_C|GetFoodExpiryElement _asbp_main_game_instance) _gameinstanceindex))
  (return _asbp_main_game_instance))

(fn EnableSlicingLevel
  (bind _outactors (Actor|GetAllActorsOfClass "/Game/TopDown/Blueprints/BP_ChangeLevelZone.BP_ChangeLevelZone_C"))
  (for _array_element _outactors
    (if (Utilities|Enum|Equal(Enum) (Utilities|GetDisplayName _array_element) "BP_ChangeLevelSlicing")
      (Rendering|SetActorHiddenInGame _array_element false)))
  (return))