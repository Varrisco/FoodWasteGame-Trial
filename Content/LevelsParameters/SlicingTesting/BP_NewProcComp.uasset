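; Sliceable food actor that supports up to 25 cuts and counts them down on screen.
; Construction copies the food's static mesh into a procedural mesh, swapping a material for bad food.
; SliceMe cuts it with a good or bad cap material, simulates physics on the new half, then fires a radial impulse and Niagara effect.
; It updates the TextRenderActor named "Counter", hiding it and flagging Slicing_Manager finished on the last cut.
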(event Custom|SliceMe
  (params (Proc%20Comp :type Procedural%20Mesh%20Component%20Object%20Reference) (Location :type Vector) (Normal :type Vector))
  (bind _radialforce (Variables|Default|GetRadialForce))
  (bind _radialforce_2 (Variables|Default|GetRadialForce))
  (if (Variables|Default|GetisBadFood)
    (bind _counter (Utilities|FlowControl|DoN 25) ; This would be useful to cut only N times.
      (:Exit
        (bind _outotherhalfprocmesh (Class|KismetProceduralMeshLibrary|SliceProceduralMesh Proc%20Comp Location Normal true "CreateNewSectionForCap" "/Game/LevelsParameters/SlicingTesting/M_BadColor.M_BadColor"))
        (Physics|SetSimulatePhysics _outotherhalfprocmesh true)
        (Collision|SetCollisionObjectType _outotherhalfprocmesh "ECC_GameTraceChannel1")
        (Transformation|SetWorldLocation _radialforce_2 Location false true)
        (Class|RadialForceComponent|FireImpulse _radialforce_2)
        (CallFunction|SetCounterText _counter)
        (AddComponent|AddNiagaraComponent false (Math|Transform|MakeTransform (Math|Vector|MakeVector 0.0 0.0 2e+01) "0, 0, 0" "1.000000,1.000000,1.000000"))
        (bind _outactors (Actor|GetAllActorsOfClass "/Game/LevelsParameters/SlicingTesting/Structures/Slicing_Manager.Slicing_Manager_C"))
        (if (== _counter 25)
          (Variables|/Game/LevelsParameters/SlicingTesting/Structures/Slicing_Manager.Slicing_Manager_C|SetFinishedCounter (Utilities|Array|Get(acopy) _outactors) true)
          (CallFunction|SetCounterInvisible)
          (else
            (Utilities|FlowControl|DoOnce false
              (:Completed
                (CallFunction|SetCounterVisible)))))))
    (else
      (bind _counter_2 (Utilities|FlowControl|DoN 25) ; This would be useful to cut only N times.
        (:Exit
          (bind _outotherhalfprocmesh_2 (Class|KismetProceduralMeshLibrary|SliceProceduralMesh Proc%20Comp Location Normal true "CreateNewSectionForCap" "/Game/LevelsParameters/SlicingTesting/M_GoodColor.M_GoodColor"))
          (Physics|SetSimulatePhysics _outotherhalfprocmesh_2 true)
          (Collision|SetCollisionObjectType _outotherhalfprocmesh_2 "ECC_GameTraceChannel1")
          (Transformation|SetWorldLocation _radialforce Location false true)
          (Class|RadialForceComponent|FireImpulse _radialforce)
          (CallFunction|SetCounterText _counter_2)
          (AddComponent|AddNiagaraComponent false (Math|Transform|MakeTransform (Math|Vector|MakeVector 0.0 0.0 2e+01) "0, 0, 0" "1.000000,1.000000,1.000000"))
          (bind _outactors_2 (Actor|GetAllActorsOfClass "/Game/LevelsParameters/SlicingTesting/Structures/Slicing_Manager.Slicing_Manager_C"))
          (if (== _counter_2 25)
            (Variables|/Game/LevelsParameters/SlicingTesting/Structures/Slicing_Manager.Slicing_Manager_C|SetFinishedCounter (Utilities|Array|Get(acopy) _outactors_2) true)
            (CallFunction|SetCounterInvisible)
            (else
              (Utilities|FlowControl|DoOnce false
                (:Completed
                  (CallFunction|SetCounterVisible))))))))))

(event EventBeginPlay)

(event Collision|EventActorBeginOverlap
  (params (OtherActor :type Actor%20Object%20Reference)))

(event EventTick
  (params (DeltaSeconds :type Float%20%28single-precision%29)))

(fn ConstructionScript
  (bind _staticmesh (Variables|Default|GetStaticMesh))
  (Components|StaticMesh|SetStaticMesh _staticmesh (Variables|/Game/LevelsParameters/SlicingTesting/Structures/SliceFoodDataAsset.SliceFoodDataAsset_C|GetMainMesh (Variables|Default|GetSliceFoodData)))
  (if (Variables|Default|GetisBadFood)
    (Rendering|Material|SetMaterial _staticmesh 1 "/Game/LevelsParameters/SlicingTesting/UnrealExample/M_BADUniversalFoodMaterial.M_BADUniversalFoodMaterial"))
  (Class|KismetProceduralMeshLibrary|CopyProceduralMeshfromStaticMeshComponent (Variables|Default|GetStaticMesh) 0 (Variables|Default|GetProceduralMesh) true)
  (Components|DestroyComponent (Variables|Default|GetStaticMesh)))

(fn SetCounterVisible
  (bind _outactors (Actor|GetAllActorsOfClass "/Script/Engine.TextRenderActor"))
  (for _array_element _outactors
    (if (Utilities|Enum|Equal(Enum) (Utilities|GetDisplayName _array_element) "Counter")
      (Rendering|SetVisibility (Variables|/Script/Engine.TextRenderActor|GetTextRender _array_element) true false)))
  (return))

(fn SetCounterInvisible
  (bind _outactors (Actor|GetAllActorsOfClass "/Script/Engine.TextRenderActor"))
  (for _array_element _outactors
    (if (Utilities|Enum|Equal(Enum) (Utilities|GetDisplayName _array_element) "Counter")
      (Rendering|SetVisibility (Variables|/Script/Engine.TextRenderActor|GetTextRender _array_element) false false)))
  (return))

(fn SetCounterText
  (params (Counter :type Integer))
  (bind _outactors (Actor|GetAllActorsOfClass "/Script/Engine.TextRenderActor"))
  (for _array_element _outactors
    (if (Utilities|Enum|Equal(Enum) (Utilities|GetDisplayName _array_element) "Counter")
      (Rendering|Components|TextRender|SetText (Variables|/Script/Engine.TextRenderActor|GetTextRender _array_element) (Utilities|Text|ToText(Integer) (- 25 Counter))))))