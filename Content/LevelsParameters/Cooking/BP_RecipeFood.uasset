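; BP_RecipeFood is a touchable food actor for cooking levels, with its mesh set from CookMeshToSet in the construction script.
; On touch it jumps to a fixed world location and, after a short delay, simulates physics so it can fall.
; After a second delay it sets Clicked and increments ClickedCooking on the CookingManager, reached through the cooking pawn cached at BeginPlay.
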(event OnInputTouchBegin(StaticMesh)
  (params (FingerIndex :type ETouchIndex%20Enum :default "Touch1") (TouchedComponent :type Primitive%20Component%20Object%20Reference))
  (Transformation|SetActorLocation "986.226500,212.681345,137.861993" false false)
  (Utilities|FlowControl|Delay 0.1)
  (Physics|SetSimulatePhysics (Variables|Default|GetStaticMesh) true)
  (Utilities|FlowControl|Delay 1.5)
  (Variables|Default|SetClicked true)
  (Math|Integer|IncrementInt (Variables|/Game/LevelsParameters/Cooking/Structures/Cooking_Manager.Cooking_Manager_C|GetClickedCooking (Variables|/Game/LevelsParameters/Cooking/CookingPawn.CookingPawn_C|GetCookingManager (Variables|Default|GetPawnRef)))))

(event EventBeginPlay
  (Utilities|IsValid (Variables|Default|GetPawnRef)
    (:Is%20Not%20Valid
      (bind _ascooking_pawn (CallFunction|GetCookingPawn))
      (Variables|Default|SetPawnRef _ascooking_pawn))))

(event Collision|EventActorBeginOverlap
  (params (OtherActor :type Actor%20Object%20Reference)))

(event EventTick
  (params (DeltaSeconds :type Float%20%28single-precision%29)))

(fn ConstructionScript
  (Components|StaticMesh|SetStaticMesh (Variables|Default|GetStaticMesh) (Variables|Default|GetCookMeshToSet)))