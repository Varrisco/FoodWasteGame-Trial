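; Slicing-level area actor that ends the cutting view and resets the slicing loop or finishes the level.
; A fast looping timer watches for Counter reaching three; that, a zone touch or TouchedUI moves the pawn out, clears the cutting flag, destroys sliced food off one exact height and shifts itself.
; AddGoodFoodAmount tallies good and bad sliced food, logging a Portuguese error and halving the good count once if any is bad.
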(event OnInputTouchBegin(ZoneMesh)
  (params (FingerIndex :type ETouchIndex%20Enum :default "Touch1") (TouchedComponent :type Primitive%20Component%20Object%20Reference))
  (CallFunction|ZoomOutTable)
  (CallFunction|ClearFoodinTable)
  (Transformation|AddLocalOffset (Variables|Default|GetDefaultSceneRoot) "1015.816352,40.274709,549.018144" false false)
  (Default|ResetLooporFinishLevel (Variables|Default|GetPawnRef)))

(event Custom|TouchedUI
  (CallFunction|ZoomOutTable)
  (CallFunction|ClearFoodinTable)
  (Transformation|AddLocalOffset (Variables|Default|GetDefaultSceneRoot) "1015.816352,40.274709,549.018144" false false)
  (Default|ResetLooporFinishLevel (Variables|Default|GetPawnRef)))

(event Custom|TimeCheckSelectedFood
  (Utilities|Time|SetTimerbyEvent (delegate Custom|CheckSelectedFood) 0.001 true))

(event Custom|CheckSelectedFood
  (if (== (Variables|Default|GetCounter) 3)
    (Variables|Default|SetCounter 0)
    (CallFunction|ZoomOutTable)
    (CallFunction|ClearFoodinTable)
    (Transformation|AddLocalOffset (Variables|Default|GetDefaultSceneRoot) "1015.816352,40.274709,549.018144" false false)
    (Default|ResetLooporFinishLevel (Variables|Default|GetPawnRef))))

(event EventBeginPlay
  ;[1 1 1] Getting a reference to storingPawn to avoid recasts
  (Utilities|IsValid (Variables|Default|GetPawnRef)
    (:Is%20Not%20Valid
      (bind _asslice_game_pawn (Utilities|Casting|CastToSliceGamePawn (Game|Player|GetPlayerPawn 0))
        (:then
          (Variables|Default|SetPawnRef _asslice_game_pawn)
          (bind _asslice_game_player_controller (Utilities|Casting|CastToSliceGamePlayerController (Game|GetPlayerController 0)))
          (Variables|Default|SetPControllerRef _asslice_game_player_controller)
          (CallFunction|TimeCheckSelectedFood))
        (:CastFailed
          (Development|PrintString "you trolling you have no storing pawn"))))))

(event Collision|EventActorBeginOverlap
  (params (OtherActor :type Actor%20Object%20Reference)))

(event EventTick
  (params (DeltaSeconds :type Float%20%28single-precision%29)))

(fn ConstructionScript)

(fn ZoomOutTable
  (Transformation|SetRelativeLocation (Variables|/Script/Engine.Actor|GetRootComponent (Variables|Default|GetPawnRef)) "560.688248,-86.345407,193.301606" false false)
  (Variables|/Game/LevelsParameters/SlicingTesting/UnrealExample/SliceGamePlayerController.SliceGamePlayerController_C|SetIsCuttingArea (Variables|Default|GetPControllerRef) false))

(fn ClearFoodinTable
  (bind _outactors (Actor|GetAllActorsOfClass "/Game/LevelsParameters/SlicingTesting/BP_SlicedFood.BP_SlicedFood_C"))
  (for _array_element _outactors
    (if (not (== (.z (Transformation|GetWorldLocation (Variables|/Game/LevelsParameters/SlicingTesting/BP_SlicedFood.BP_SlicedFood_C|GetProceduralMesh _array_element))) 137.861993))
      (Actor|DestroyActor _array_element))))

(fn AddGoodFoodAmount
  (bind _outactors (Actor|GetAllActorsOfClass "/Game/LevelsParameters/SlicingTesting/BP_SlicedFood.BP_SlicedFood_C"))
  (for _array_element _outactors
    (if (Variables|/Game/LevelsParameters/SlicingTesting/BP_SlicedFood.BP_SlicedFood_C|GetisBadFood _array_element)
      (Math|Integer|IncrementInt (Variables|Default|GetBadFoodSelected))
      (else
        (Math|Integer|IncrementInt (Variables|Default|GetGoodFoodSelected)))))
  (if (!= (Variables|Default|GetBadFoodSelected) 0)
    (Utilities|FlowControl|DoOnce false
      (:Completed
        (Default|AddErrors (Variables|/Game/LevelsParameters/SlicingTesting/UnrealExample/SliceGamePawn.SliceGamePawn_C|GetSlicingComponent (Variables|Default|GetPawnRef)) (Utilities|String|ToString(Text) (Utilities|Text|FormatText "Selecionas-te {number} comida(s) má para cozinhar;" (Variables|Default|GetBadFoodSelected))))
        (Variables|Default|SetGoodFoodSelected (/ (Variables|Default|GetGoodFoodSelected) 2)))))
  (return (Variables|Default|GetGoodFoodSelected)))